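; BP_GrenadeProjectile is a timed grenade actor that explodes and deals area damage.
; BeginPlay starts a short fuse delay, then calls the Explode event.
; Explode spawns the explosion particle, applies radial damage without falloff credited to the instigator's controller, and destroys the actor.
; It also draws a debug sphere matching the damage radius to visualize the hit area.
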(event Custom|Explode
  (bind _returnvalue (Transformation|GetActorLocation))
  ;[1 0.1744 0.58] Apply damage and draws a sphere for show radial hit
  (Effects|SpawnEmitteratLocation "/Game/StarterContent/Particles/P_Explosion.P_Explosion" _returnvalue)
  (Game|Damage|ApplyRadialDamage 1e+02 _returnvalue (Variables|Default|GetDamageRadius) 0 0 self (Game|GetInstigatorController) true "ECC_Visibility")
  (Actor|DestroyActor)
  (Rendering|Debug|DrawDebugSphere _returnvalue (Variables|Default|GetDamageRadius) 12 "(R=1.000000,G=0.672742,B=0.000000,A=1.000000)" 1.0 2.0))

(event EventBeginPlay
  ;[0.2621 1 0.4888] Calls the function Explode with a delay of 1 sec
  (Utilities|FlowControl|Delay 1.0)
  (CallFunction|Explode))

(fn ConstructionScript)